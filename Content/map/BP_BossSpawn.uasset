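; Boss spawn point that creates BP_Enemy encounters from a random entry in its SpawnType array.
; When NewEnemyfromSpawnType fires, it rolls one of two enemy attributes, activates a Niagara effect and spawns after a short delay.
; Gemini Rotating and Turrent types spawn offset pairs linked to each other through RelyActor, then destroy the spawner.
; Charger spawns a single enemy at the spawner's location and leaves the spawner in place.
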(event `self.NewEnemyFromSpawnType`
  (bind _returnvalue (`self.K2_GetActorLocation`))
  (bind _returnvalue_2 (`self.K2_GetActorLocation`))
  (bind _niagara (`self.Niagara`))
  (bind _niagara_2 (`self.Niagara`))
  (bind _attribute (`self.Attribute`))
  (bind _niagara_3 (`self.Niagara`))
  (bind _spawntype (`self.SpawnType`))
  (bind _attribute_2 (`self.Attribute`))
  (`|ExecutionSequence`
    (:`then_0`
      (switch `int` (`KismetMathLibrary.RandomIntegerInRange` 0 1)
        (:`Default`
          (set `self.Attribute` "NewEnumerator2" :!label _label))
        (:`0`
          (set `self.Attribute` "NewEnumerator0"))
        (:`1`
          (set `self.Attribute` "NewEnumerator1"))
        (:`2`
          (goto _label))))
    (:`then_1`
      (bind _output_get (set `self.type` (`|GetArrayItem` _spawntype (`KismetMathLibrary.RandomIntegerInRange` 0 (- (`KismetArrayLibrary.Array_Length` _spawntype) 1)))))
      (switch `/Game/util/EnemyType` _output_get
        (:`NewEnumerator2`
          (`/Engine/EditorBlueprintResources/StandardMacros.IsValid` _niagara_3
            (:`Is Valid`
              (`ActorComponent.SetActive` _niagara_3 true false)
              (`KismetSystemLibrary.Delay` 2.0)
              (bind _returnvalue_3 (`|SpawnActorFromClass` "/Game/enemy/BP_Enemy.BP_Enemy_C" (`KismetMathLibrary.MakeTransform` (- _returnvalue (0.0 150.0 0.0))) "AdjustIfPossibleButAlwaysSpawn" "OverrideRootScale" null _attribute_2 "NewEnumerator2" false false null null))
              (bind _output_get_2 (set `self.temp` _returnvalue_3))
              (bind _returnvalue_4 (`|SpawnActorFromClass` "/Game/enemy/BP_Enemy.BP_Enemy_C" (`KismetMathLibrary.MakeTransform` (+ _returnvalue (0.0 150.0 0.0))) "AdjustIfPossibleButAlwaysSpawn" "OverrideRootScale" null _attribute_2 "NewEnumerator2" false true _output_get_2 null))
              (set `/Game/enemy/BP_Enemy.RelyActor` _returnvalue_4 _output_get_2)
              (`KismetSystemLibrary.Delay` 0.2)
              (`self.K2_DestroyActor`))))
        (:`NewEnumerator3`
          (`/Engine/EditorBlueprintResources/StandardMacros.IsValid` _niagara_2
            (:`Is Valid`
              (`ActorComponent.SetActive` _niagara_2 true false)
              (`KismetSystemLibrary.Delay` 2.0)
              (bind _returnvalue_5 (`|SpawnActorFromClass` "/Game/enemy/BP_Enemy.BP_Enemy_C" (`KismetMathLibrary.MakeTransform` (- _returnvalue_2 (0.0 100.0 0.0))) "AdjustIfPossibleButAlwaysSpawn" "OverrideRootScale" null _attribute "NewEnumerator3" false true null null))
              (bind _output_get_3 (set `self.temp` _returnvalue_5))
              (bind _returnvalue_6 (`|SpawnActorFromClass` "/Game/enemy/BP_Enemy.BP_Enemy_C" (`KismetMathLibrary.MakeTransform` (+ _returnvalue_2 (0.0 100.0 0.0))) "AdjustIfPossibleButAlwaysSpawn" "OverrideRootScale" null _attribute "NewEnumerator3" false true _output_get_3 null))
              (set `/Game/enemy/BP_Enemy.RelyActor` _returnvalue_6 _output_get_3)
              (`KismetSystemLibrary.Delay` 0.2)
              (`self.K2_DestroyActor`))))
        (:`NewEnumerator4`
          (`/Engine/EditorBlueprintResources/StandardMacros.IsValid` _niagara
            (:`Is Valid`
              (`ActorComponent.SetActive` _niagara true false)
              (`KismetSystemLibrary.Delay` 2.0)
              (`|SpawnActorFromClass` "/Game/enemy/BP_Enemy.BP_Enemy_C" (`KismetMathLibrary.MakeTransform` (`self.K2_GetActorLocation`)) "AdjustIfPossibleButAlwaysSpawn" "OverrideRootScale" null (`self.Attribute`) "NewEnumerator4" false false null null))))))))

(fn `UserConstructionScript`
  (`parent.UserConstructionScript`))