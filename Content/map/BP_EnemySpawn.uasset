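; BP_EnemySpawn is a one-shot spawn point that usually creates a randomized BP_Enemy at its location on BeginPlay.
; A random roll can skip spawning; otherwise it picks one of two attributes, a type from the SpawnType array, and an occasional violent flag.
; NewEnemy activates a Niagara effect, spawns the enemy after a short delay, then destroys the spawner.
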(event `self.ReceiveBeginPlay`
  (`self.NewEnemyFromSpawnType`))

(event `New Enemy`
  (params (EnemyAttribute :type "/Game/util/Attribute Enum" :default "NewEnumerator0") (EnemyType :type "/Game/util/EnemyType Enum" :default "NewEnumerator0") (isReliable :type Boolean) (RelyActor :type "/Game/enemy/BP_Enemy Object Reference") (isViolent :type Boolean) (SpawnTransform :type "Transform Structure"))
  (bind _niagara (`self.Niagara`))
  (`/Engine/EditorBlueprintResources/StandardMacros.IsValid` _niagara
    (:`Is Valid`
      (`ActorComponent.SetActive` _niagara true false)
      (`KismetSystemLibrary.Delay` 1.0)
      (`|SpawnActorFromClass` "/Game/enemy/BP_Enemy.BP_Enemy_C" SpawnTransform "AdjustIfPossibleButAlwaysSpawn" "OverrideRootScale" null EnemyAttribute EnemyType isViolent isReliable RelyActor null)
      (`KismetSystemLibrary.Delay` 0.2)
      (`self.K2_DestroyActor`))))

(event `NewEnemyFromSpawnType`
  (bind _spawntype (`self.SpawnType`))
  (if (<= (`KismetMathLibrary.RandomIntegerInRange` 0 8) 7)
    (`|ExecutionSequence`
      (:`then_0`
        (switch `int` (`KismetMathLibrary.RandomIntegerInRange` 0 1)
          (:`Default`
            (set `self.Attribute` "NewEnumerator2" :!label _label))
          (:`0`
            (set `self.Attribute` "NewEnumerator0"))
          (:`1`
            (set `self.Attribute` "NewEnumerator1"))
          (:`2`
            (goto _label))))
      (:`then_1`
        (if (<= (`KismetMathLibrary.RandomIntegerInRange` 0 8) 1)
          (set `self.Violent` true)
          (else
            (set `self.Violent` false))))
      (:`then_2`
        (set `self.type` (`|GetArrayItem` _spawntype (`KismetMathLibrary.RandomIntegerInRange` 0 (- (`KismetArrayLibrary.Array_Length` _spawntype) 1)))))
      (:`then_3`
        (`self.New Enemy` (`self.Attribute`) (`self.type`) false null (`self.Violent`) (`KismetMathLibrary.MakeTransform` (`self.K2_GetActorLocation`)))))))

(fn `UserConstructionScript`)