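; Enemy bomb projectile that explodes after a telegraphed delay once it touches the player, a static mesh actor or another enemy.
; Contact freezes its physics and spawns an AOE decal, whose dynamic material a timeline animates as a warning.
; An outer sphere tracks whether the player is in range; when the timeline ends, they take data-table damage if still inside.
; The bomb then plays burst FX and distance-scaled sound before destroying itself.
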(event `self.ReceiveBeginPlay`)

(event `self.Sphere.OnComponentBeginOverlap`
  (params (OverlappedComponent :type "PrimitiveComponent Object Reference") (OtherActor :type "Actor Object Reference") (OtherComp :type "PrimitiveComponent Object Reference") (OtherBodyIndex :type Integer) (bFromSweep :type Boolean) (SweepResult :type "HitResult Structure (by ref)"))
  (cast `/Game/character/BP_Character` OtherActor
    (:`then`
      _)
    (:`CastFailed`
      (cast `StaticMeshActor` OtherActor
        (:`then`
          _)
        (:`CastFailed`
          (cast `/Game/enemy/BP_Enemy` OtherActor)))))
  (`self.Boom`))

(event `Boom`
  (bind _returnvalue (`self.K2_GetActorLocation`))
  (if (not (`self.isBoomed`))
    (set `self.isBoomed` true)
    (`PrimitiveComponent.SetSimulatePhysics` (`self.Cube`) false)
    (bind _returnvalue_2 (`GameplayStatics.SpawnDecalAtLocation` "/Game/material/M_RoundAOE.M_RoundAOE" (128.0 256.0 256.0) (`self.K2_GetActorLocation`)))
    (bind _output_get (set `self.Decal` _returnvalue_2))
    (`DecalComponent.SetDecalMaterial` _output_get (`self.Material`))
    (bind (_direction _hint) (`Timeline|Hint`)
      (:`Update`
        (`MaterialInstanceDynamic.SetScalarParameterValue` (`self.Material`) "Time" _hint))
      (:`Finished`
        (`|ExecutionSequence`
          (:`then_0`
            (if (`self.hit`)
              (bind _returnvalue_3 (`|GetDataTableRow` "/Game/util/WeaponDataTable.WeaponDataTable" "BoomEnemy")
                (:`then`
                  (`GameplayStatics.ApplyDamage` (`GameplayStatics.GetPlayerCharacter` 0) (`.damage_10_C9277D9B4CC62D6798D0FABC4F40C1BC` (break `/Game/util/WeaponInfo` _returnvalue_3)) null null "/Game/util/DamageTypeRedBoom.DamageTypeRedBoom_C")))))
          (:`then_1`
            (`NiagaraFunctionLibrary.SpawnSystemAtLocation` "/Game/particlesystem/FX_burstSystem.FX_burstSystem" _returnvalue)
            (`GameplayStatics.PlaySoundAtLocation` "/Game/Retro_8Bit_Sounds/Explosion/Cues/retro_explosion_bass_03_Cue.retro_explosion_bass_03_Cue" _returnvalue (struct) (`KismetMathLibrary.FMin` (/ 600.0 (`KismetMathLibrary.VSize` (- _returnvalue (`self.K2_GetActorLocation` (`GameplayStatics.GetPlayerCharacter` 0))))) 1.0) 1.0 0.0 null null null))
          (:`then_2`
            (`ActorComponent.K2_DestroyComponent` (`self.Decal`))
            (`self.K2_DestroyActor`)))))))

(event `self.SphereBoom.OnComponentBeginOverlap`
  (params (OverlappedComponent :type "PrimitiveComponent Object Reference") (OtherActor :type "Actor Object Reference") (OtherComp :type "PrimitiveComponent Object Reference") (OtherBodyIndex :type Integer) (bFromSweep :type Boolean) (SweepResult :type "HitResult Structure (by ref)"))
  (cast `/Game/character/BP_Character` OtherActor)
  (set `self.hit` true))

(event `self.SphereBoom.OnComponentEndOverlap`
  (params (OverlappedComponent :type "PrimitiveComponent Object Reference") (OtherActor :type "Actor Object Reference") (OtherComp :type "PrimitiveComponent Object Reference") (OtherBodyIndex :type Integer))
  (cast `/Game/character/BP_Character` OtherActor)
  (set `self.hit` false))

(fn `UserConstructionScript`
  (bind _returnvalue (`KismetMaterialLibrary.CreateDynamicMaterialInstance` "/Game/material/M_RoundAOE.M_RoundAOE"))
  (set `self.Material` _returnvalue))