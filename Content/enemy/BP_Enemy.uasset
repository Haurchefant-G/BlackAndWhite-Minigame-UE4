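; All-in-one enemy character for artillery, infantry, charger and twin Gemini bosses, each in a White or Black polarity.
; Construction applies type visuals and data-table stats; BeginPlay buffs violent elites and starts a type-specific behavior tree.
; Skills provide bullets, radial rings and telegraphed trace lasers, while chargers deal speed-scaled contact damage.
; Only opposite-polarity bullets or lasers hurt it, Gemini state follows RelyActor validity, and death awards score and dissolves it.
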(event `self.ReceiveBeginPlay`
  (bind _enemyattribute (`self.EnemyAttribute`))
  (bind _mesh (`self.Mesh`))
  (bind _returnvalue (`AIBlueprintHelperLibrary.GetAIController` self))
  (bind (_returnvalue_location _returnvalue_rotation _returnvalue_scale) (`KismetMathLibrary.BreakTransform` (`SceneComponent.GetRelativeTransform` _mesh)))
  ;[1 1 1] 开场 精英怪强化 行为树选择
  (`|ExecutionSequence`
    (:`then_0`
      (if (`self.isViolent`)
        (set `self.maxhp` (* (`self.maxhp`) (`self.hpStrengthenRating`)))
        (set `self.damageRating` (+ (`self.damageRating`) 0.5))
        (set `self.InitBulletSize` (* (`self.InitBulletSize`) 1.5))
        (`SceneComponent.K2_SetRelativeTransform` _mesh (`KismetMathLibrary.MakeTransform` _returnvalue_location _returnvalue_rotation (* _returnvalue_scale 1.5)) false false)))
    (:`then_1`
      (switch `/Game/util/EnemyType` (`self.EnemyType`)
        (:`NewEnumerator0`
          (`KismetSystemLibrary.Delay` (`KismetMathLibrary.RandomFloatInRange` 0.5 1.5))
          (`AIController.UseBlackboard` _returnvalue "/Game/AI/PlayerBlackboardData.PlayerBlackboardData")
          (switch `int` (`KismetMathLibrary.RandomIntegerInRange` 0 3)
            (:`Default`
              (`AIController.RunBehaviorTree` _returnvalue "/Game/AI/TurrentBehaviorTreeBullet.TurrentBehaviorTreeBullet" :!label _label))
            (:`0`
              (if (`|EnumEquality` _enemyattribute "NewEnumerator0")
                (`AIController.RunBehaviorTree` _returnvalue "/Game/AI/TurrentBehaviorTreeLaser.TurrentBehaviorTreeLaser")
                (else
                  (goto _label))))
            (:`1`
              (goto _label))
            (:`2`
              (goto _label))))
        (:`NewEnumerator1`
          (`KismetSystemLibrary.Delay` (`KismetMathLibrary.RandomFloatInRange` 0.5 1.5))
          (`AIController.UseBlackboard` _returnvalue "/Game/AI/PlayerBlackboardData.PlayerBlackboardData")
          (switch `int` (`KismetMathLibrary.RandomIntegerInRange` 0 3)
            (:`Default`
              (`AIController.RunBehaviorTree` _returnvalue "/Game/AI/ChaseBehaviorTreeBullet.ChaseBehaviorTreeBullet" :!label _label_2))
            (:`0`
              (if (`|EnumEquality` _enemyattribute "NewEnumerator0")
                (`AIController.RunBehaviorTree` _returnvalue "/Game/AI/ChaseBehaviorTreeLaser.ChaseBehaviorTreeLaser")
                (else
                  (goto _label_2))))
            (:`1`
              (goto _label_2))
            (:`2`
              (goto _label_2))))
        (:`NewEnumerator2`
          (`KismetSystemLibrary.Delay` (`KismetMathLibrary.RandomFloatInRange` 0.5 1.5))
          (`AIController.UseBlackboard` _returnvalue "/Game/AI/PlayerBlackboardData.PlayerBlackboardData")
          (`AIController.RunBehaviorTree` _returnvalue "/Game/AI/BehaviorTreeGeminiRotating.BehaviorTreeGeminiRotating"))
        (:`NewEnumerator3`
          (`KismetSystemLibrary.Delay` (`KismetMathLibrary.RandomFloatInRange` 0.5 1.5))
          (`AIController.UseBlackboard` _returnvalue "/Game/AI/PlayerBlackboardData.PlayerBlackboardData")
          (`AIController.RunBehaviorTree` _returnvalue "/Game/AI/BehaviorTreeGeminiTurrent.BehaviorTreeGeminiTurrent"))
        (:`NewEnumerator4`
          (`KismetSystemLibrary.Delay` (`KismetMathLibrary.RandomFloatInRange` 0.5 1.5))
          (`AIController.UseBlackboard` _returnvalue "/Game/AI/PlayerBlackboardData.PlayerBlackboardData")
          (`AIController.RunBehaviorTree` _returnvalue "/Game/AI/BehaviorTreeCharger.BehaviorTreeCharger")
          (add `PrimitiveComponent.OnComponentBeginOverlap` (`self.Sphere`) (delegate `OnCharge`)))))))

(event `OnCharge`
  (params (OverlappedComponent :type "PrimitiveComponent Object Reference") (OtherActor :type "Actor Object Reference") (OtherComp :type "PrimitiveComponent Object Reference") (OtherBodyIndex :type Integer) (bFromSweep :type Boolean) (SweepResult :type "HitResult Structure (by ref)"))
  ;[1 1 1] 冲撞的碰撞事件
  (bind _asbp_character (cast `/Game/character/BP_Character` OtherActor))
  (bind _returnvalue (`|GetDataTableRow` "/Game/util/WeaponDataTable.WeaponDataTable" "Charger")
    (:`then`
      (switch `/Game/util/Attribute` (`self.EnemyAttribute`)
        (:`NewEnumerator0`
          (bind _returnvalue_2 (* (`.damage_10_C9277D9B4CC62D6798D0FABC4F40C1BC` (break `/Game/util/WeaponInfo` _returnvalue)) (`self.damageRating`)))
          (bind _returnvalue_3 (`KismetMathLibrary.FMax` (* _returnvalue_2 (/ (`KismetMathLibrary.VSize` (`self.GetVelocity`)) (`CharacterMovementComponent.MaxWalkSpeed` (`self.CharacterMovement`)))) (* _returnvalue_2 0.2)))
          (`GameplayStatics.ApplyDamage` _asbp_character _returnvalue_3 null self "/Game/util/DamageTypeWhiteCharger.DamageTypeWhiteCharger_C"))
        (:`NewEnumerator1`
          (`GameplayStatics.ApplyDamage` _asbp_character _returnvalue_3 null self "/Game/util/DamageTypeBlackCharger.DamageTypeBlackCharger_C"))))))

(event `self.ReceiveTick`
  (params (DeltaSeconds :type "Float (single-precision)"))
  (bind _charactermovement (`self.CharacterMovement`))
  ;[1 1 1] 每帧判断
  (if (not (`self.isDead`))
    (switch `/Game/util/EnemyType` (`self.EnemyType`)
      (:`NewEnumerator2`
        (if (`self.isReliable`)
          (`/Engine/EditorBlueprintResources/StandardMacros.IsValid` (`self.RelyActor`)
            (:`Is Valid`
              (`/Engine/EditorBlueprintResources/StandardMacros.DoOnce` false
                (:`Completed`
                  (set `self.canMove` false)
                  (set `self.canbehurt` false))))
            (:`Is Not Valid`
              (`/Engine/EditorBlueprintResources/StandardMacros.DoOnce` false
                (:`Completed`
                  (set `self.isViolent` true)
                  (set `self.canbehurt` true)
                  (set `self.canMove` true)))))
          (else
            (`/Engine/EditorBlueprintResources/StandardMacros.DoOnce` false
              (:`Completed`
                (set `self.canbehurt` true))))))
      (:`NewEnumerator3`
        (`/Engine/EditorBlueprintResources/StandardMacros.IsValid` (`self.RelyActor`)
          (:`Is Valid`
            (`/Engine/EditorBlueprintResources/StandardMacros.DoOnce` false
              (:`Completed`
                (set `self.canMove` false)
                (set `self.canbehurt` true))))
          (:`Is Not Valid`
            (`/Engine/EditorBlueprintResources/StandardMacros.DoOnce` false
              (:`Completed`
                (set `self.isViolent` true)
                (set `self.canbehurt` true)
                (set `self.canMove` true))))))
      (:`NewEnumerator4`
        (if (< (`self.hp`) (* (`self.maxhp`) 0.5))
          (set `self.isViolent` true)
          (set `CharacterMovementComponent.MaxWalkSpeed` (* (`CharacterMovementComponent.MaxWalkSpeed` _charactermovement) 1.5) _charactermovement))))))

(event `self.ReceiveAnyDamage`
  (params (Damage :type "Float (single-precision)") (DamageType :type "DamageType Object Reference") (InstigatedBy :type "Controller Object Reference") (DamageCauser :type "Actor Object Reference"))
  (bind _enemyattribute (`self.EnemyAttribute`))
  ;[1 1 1] 伤害事件
  (if (`self.canbehurt`)
    (cast `/Game/util/DamageTypeBlackBullet` DamageType
      (:`then`
        (switch `/Game/util/Attribute` _enemyattribute
          (:`NewEnumerator0`
            (`self.getDamage` Damage))))
      (:`CastFailed`
        (cast `/Game/util/DamageTypeWhiteLaser` DamageType)
        (switch `/Game/util/Attribute` _enemyattribute
          (:`NewEnumerator1`
            (`self.getDamage` Damage)))))))

(event `death`
  (bind _deadmaterial (`self.deadMaterial`))
  (bind _mesh (`self.Mesh`))
  (bind _deadmaterial_2 (`self.deadMaterial`))
  (bind _mesh_2 (`self.Mesh`))
  ;[1 1 1] 死亡事件
  (set `self.isDead` true)
  (bind _asbp_character (cast `/Game/character/BP_Character` (`GameplayStatics.GetPlayerCharacter` 0))
    (:`then`
      (set `/Game/character/BP_Character.score` (+ (`/Game/character/BP_Character.score` _asbp_character) (`self.maxhp`)) _asbp_character))
    (:`CastFailed`
      _))
  (`self.SetActorEnableCollision` false)
  (switch `/Game/util/EnemyType` (`self.EnemyType`)
    (:`NewEnumerator0`
      (`PrimitiveComponent.SetMaterial` _mesh 0 _deadmaterial_2 :!label _label_3)
      (`PrimitiveComponent.SetMaterial` _mesh 1 _deadmaterial_2)
      (bind (_direction _deathdelta) (`Timeline|deathTimeline` :!label _label_4)
        (:`Update`
          (`MaterialInstanceDynamic.SetScalarParameterValue` (`self.deadMaterial`) "time" _deathdelta))
        (:`Finished`
          (`Widget.RemoveFromParent` (`self.DamageUI`))
          (`self.K2_DestroyActor`))))
    (:`NewEnumerator1`
      (goto _label_3))
    (:`NewEnumerator2`
      (`PrimitiveComponent.SetMaterial` _mesh_2 0 _deadmaterial :!label _label_5)
      (`PrimitiveComponent.SetMaterial` _mesh_2 1 _deadmaterial)
      (`PrimitiveComponent.SetMaterial` _mesh_2 2 _deadmaterial)
      (`PrimitiveComponent.SetMaterial` _mesh_2 3 _deadmaterial)
      (goto _label_4))
    (:`NewEnumerator3`
      (goto _label_5))
    (:`NewEnumerator4`
      (`PrimitiveComponent.SetMaterial` (`self.Mesh`) 0 (`self.deadMaterial`))
      (goto _label_4))))

(fn `getDamage`
  (params (damage :type "Float (double-precision)"))
  (bind _returnvalue (`self.K2_GetActorLocation`))
  (bind _returnvalue_2 (`KismetStringLibrary.Conv_DoubleToString` damage))
  (bind _damageui (`self.DamageUI`))
  (bind _damageui_2 (`self.DamageUI`))
  (bind _screenposition (`GameplayStatics.ProjectWorldToScreen` (`GameplayStatics.GetPlayerController` 0) (`self.K2_GetActorLocation`)))
  (`NiagaraFunctionLibrary.SpawnSystemAtLocation` "/Game/particlesystem/FX_hitSystem.FX_hitSystem" _returnvalue)
  (`GameplayStatics.PlaySoundAtLocation` "/Game/Retro_8Bit_Sounds/Impacts/Wavs/Damage.Damage" _returnvalue (struct) 1.0 1.0 0.0 null null null)
  (bind _output_get (set `self.hp` (- (`self.hp`) damage)))
  (if (<= _output_get 0.0)
    (`self.death`)
    (else
      (`/Engine/EditorBlueprintResources/StandardMacros.IsValid` _damageui
        (:`Is Valid`
          (set `/Game/UI/UMG_Damage.damage` _returnvalue_2 _damageui)
          (`UserWidget.SetPositionInViewport` _damageui_2 _screenposition true)
          (`/Game/UI/UMG_Damage.appear` _damageui_2))
        (:`Is Not Valid`
          (bind _returnvalue_3 (`|CreateWidget` "/Game/UI/UMG_Damage.UMG_Damage_C" (`GameplayStatics.GetPlayerController` 0)))
          (bind _output_get_2 (set `self.DamageUI` _returnvalue_3))
          (set `/Game/UI/UMG_Damage.damage` _returnvalue_2 _output_get_2)
          (`UserWidget.AddToViewport` _returnvalue_3 0)
          (`UserWidget.SetPositionInViewport` _output_get_2 _screenposition true)
          (`/Game/UI/UMG_Damage.appear` _output_get_2))))))

(fn `SkillEmmitBullet`
  (params (direction :type "Vector Structure"))
  (locals (currentDamage :type "Float (double-precision)"))
  (bind _returnvalue (`KismetMathLibrary.Conv_VectorToRotator` direction))
  (bind _currentdamage (`local.currentDamage`))
  (bind _returnvalue_2 (+ (`SceneComponent.K2_GetComponentLocation` (`self.CapsuleComponent`)) (`KismetMathLibrary.GreaterGreater_VectorRotator` (`self.GunOffset`) _returnvalue)))
  (bind _returnvalue_3 (`KismetMathLibrary.MakeTransform` _returnvalue_2 _returnvalue (`self.InitBulletSize`)))
  (if (and (> (`KismetMathLibrary.VSize` direction) 0.0) (not (`self.isDead`)))
    (bind _returnvalue_4 (`|GetDataTableRow` "/Game/util/WeaponDataTable.WeaponDataTable" "GunEnemy")
      (:`then`
        (if (`self.isViolent`)
          (bind (_weapontype _firerate _mpinfluence _damage) (break `/Game/util/WeaponInfo` _returnvalue_4))
          (set `local.currentDamage` (* _damage (+ (`self.damageRating`) 0.5)))
          (else
            (set `local.currentDamage` _damage)))
        (switch `/Game/util/Attribute` (`self.EnemyAttribute`)
          (:`NewEnumerator0`
            (`|SpawnActorFromClass` "/Game/enemy/BP_EnemyBulletWhite.BP_EnemyBulletWhite_C" _returnvalue_3 "AlwaysSpawn" "OverrideRootScale" null _currentdamage null))
          (:`NewEnumerator1`
            (`|SpawnActorFromClass` "/Game/enemy/BP_EnemyBulletBlack.BP_EnemyBulletBlack_C" _returnvalue_3 "AlwaysSpawn" "OverrideRootScale" null _currentdamage null)))
        (`GameplayStatics.PlaySoundAtLocation` "/Engine/VREditor/Sounds/UI/Click_on_Button.Click_on_Button" _returnvalue_2 (struct) 1.0 1.0 0.0 null null null)))))

(fn `SkillEmmitLaser`
  (params (direction :type "Vector Structure"))
  (bind _output_get (set `self.CurrentDirection` direction))
  (if (and (> (`KismetMathLibrary.VSize` _output_get) 0.0) (not (`self.isDead`)))
    (bind _returnvalue (`|GetDataTableRow` "/Game/util/WeaponDataTable.WeaponDataTable" "LaserEnemy")
      (:`then`
        (if (`self.isViolent`)
          (bind (_weapontype _firerate _mpinfluence _damage _range) (break `/Game/util/WeaponInfo` _returnvalue))
          (set `self.currentLaserDamage` (* _damage (+ (`self.damageRating`) 0.5)))
          (else
            (set `self.currentLaserDamage` _damage)))
        (`NiagaraFunctionLibrary.SpawnSystemAtLocation` "/Game/particlesystem/FX_Lasernotice_System.FX_Lasernotice_System" (`SceneComponent.K2_GetComponentLocation` (`self.CapsuleComponent`)) (`KismetMathLibrary.Conv_VectorToRotator` _output_get))
        (`KismetSystemLibrary.K2_SetTimer` null "SkillEmmitLaser2" 0.5)))))

(fn `SkillEmmitLaser2`
  (locals (range :type "Float (double-precision)" :default 400.0))
  (bind _returnvalue (`SceneComponent.K2_GetComponentLocation` (`self.CapsuleComponent`)))
  (bind _returnvalue_2 (`KismetMathLibrary.Conv_VectorToRotator` (`self.CurrentDirection`)))
  (`NiagaraFunctionLibrary.SpawnSystemAtLocation` "/Game/particlesystem/FX_LaserSystemEnemy.FX_LaserSystemEnemy" _returnvalue _returnvalue_2)
  (bind _outhits (`KismetSystemLibrary.LineTraceMulti` :`Start` _returnvalue :`End` (+ _returnvalue (* (`KismetMathLibrary.GetForwardVector` _returnvalue_2) (`local.range`))) :`TraceChannel` "TraceTypeQuery2" :`DrawTime` 2.0))
  (for _array_element _outhits
    (bind _asbp_character (cast `/Game/character/BP_Character` (`.HitActor` (`GameplayStatics.BreakHitResult` _array_element))))
    (`GameplayStatics.ApplyDamage` _asbp_character (`self.currentLaserDamage`) null (`self.GetController`) "/Game/util/DamageTypeWhiteLaser.DamageTypeWhiteLaser_C"))
  (`GameplayStatics.PlaySoundAtLocation` "/Engine/VREditor/Sounds/UI/Click_on_Button.Click_on_Button" (0.0 0.0 0.0) (struct) 1.0 1.0 0.0 null null null))

(fn `SkillUltimateRing`
  (params (fragment :type Integer))
  (locals (i :type Integer) (currentDamage :type "Float (double-precision)"))
  (bind _currentdamage (`local.currentDamage`))
  (bind _returnvalue (* (`local.i`) (/ 360.0 (`KismetMathLibrary.Conv_IntToDouble` fragment))))
  (bind _returnvalue_2 (`KismetMathLibrary.MakeVector` (* 1 (`KismetMathLibrary.DegCos` _returnvalue)) (* 1 (`KismetMathLibrary.DegSin` _returnvalue))))
  (bind _returnvalue_3 (+ (`SceneComponent.K2_GetComponentLocation` (`self.CapsuleComponent`)) (`KismetMathLibrary.GreaterGreater_VectorRotator` (`self.GunOffset`) (`KismetMathLibrary.Conv_VectorToRotator` _returnvalue_2))))
  (bind _returnvalue_4 (`KismetMathLibrary.MakeTransform` _returnvalue_3 (`KismetMathLibrary.Conv_VectorToRotator` _returnvalue_2) (`self.InitBulletSize`)))
  (if (not (`self.isDead`))
    (bind _returnvalue_5 (`|GetDataTableRow` "/Game/util/WeaponDataTable.WeaponDataTable" "UltimateRing")
      (:`then`
        (set `local.currentDamage` (* (`.damage_10_C9277D9B4CC62D6798D0FABC4F40C1BC` (break `/Game/util/WeaponInfo` _returnvalue_5)) (+ (`self.damageRating`) 0.5)))
        (for _index (range 1 (+ fragment 1))
          (set `local.i` _index)
          (switch `/Game/util/Attribute` (`self.EnemyAttribute`)
            (:`NewEnumerator0`
              (`|SpawnActorFromClass` "/Game/enemy/BP_EnemyBulletWhite.BP_EnemyBulletWhite_C" _returnvalue_4 "AlwaysSpawn" "OverrideRootScale" null _currentdamage null))
            (:`NewEnumerator1`
              (`|SpawnActorFromClass` "/Game/enemy/BP_EnemyBulletBlack.BP_EnemyBulletBlack_C" _returnvalue_4 "AlwaysSpawn" "OverrideRootScale" null _currentdamage null))))
        (`GameplayStatics.PlaySoundAtLocation` "/Engine/VREditor/Sounds/UI/Flashlight_Switch.Flashlight_Switch" _returnvalue_3 (struct) 1.0 1.0 0.0 null null null)))))

(fn `UserConstructionScript`
  (bind _mesh (`self.Mesh`))
  (bind _normalmaterial (`self.normalMaterial`))
  (bind _mesh_2 (`self.Mesh`))
  (bind _normalmaterial_2 (`self.normalMaterial`))
  (bind _normalmaterial_3 (`self.normalMaterial`))
  (bind _mesh_3 (`self.Mesh`))
  (bind _normalmaterial_4 (`self.normalMaterial`))
  (bind _normalmaterial_5 (`self.normalMaterial`))
  (bind _normalmaterial_6 (`self.normalMaterial`))
  (bind _normalmaterial_7 (`self.normalMaterial`))
  (bind _mesh_4 (`self.Mesh`))
  (bind _normalmaterial_8 (`self.normalMaterial`))
  (bind _returnvalue (`KismetMaterialLibrary.CreateDynamicMaterialInstance` "/Game/material/M_PureColor_Black.M_PureColor_Black"))
  (set `self.normalMaterial` _returnvalue)
  (bind _returnvalue_2 (`KismetMaterialLibrary.CreateDynamicMaterialInstance` "/Game/material/Dissolution_2.Dissolution_2"))
  (set `self.deadMaterial` _returnvalue_2)
  (switch `/Game/util/EnemyType` (`self.EnemyType`)
    (:`NewEnumerator0`
      (`SkinnedMeshComponent.SetSkinnedAssetAndUpdate` _mesh_4 "/Game/mesh/enemy2.enemy2" true)
      (`SkeletalMeshComponent.SetAnimInstanceClass` _mesh_4 "/Game/mesh/enemy2_Skeleton_AnimBlueprint.enemy2_Skeleton_AnimBlueprint_C")
      (`SceneComponent.K2_SetRelativeLocation` _mesh_4 (0.0 0.0 -30.0) false false)
      (switch `/Game/util/Attribute` (`self.EnemyAttribute`)
        (:`NewEnumerator0`
          (`MaterialInstanceDynamic.SetVectorParameterValue` _normalmaterial "color" (struct :`R` 0.99 :`G` 0.99 :`B` 0.99 :`A` 1.0))
          (`PrimitiveComponent.SetMaterial` _mesh_4 0 _normalmaterial)
          (`PrimitiveComponent.SetMaterial` _mesh_4 1 "/Game/material/材质_003.材质_003")
          (bind _returnvalue_3 (`|GetDataTableRow` "/Game/util/EnemyDataTable.EnemyDataTable" "artilleryW")
            (:`then`
              (bind (_type _maxhp _maxmp _attribute _maxvelocity _damagerating) (break `/Game/util/EnemyInfo` _returnvalue_3))
              (bind _output_get (set `self.maxhp` _maxhp))
              (set `self.hp` _output_get)
              (set `self.maxmp` _maxmp)
              (set `CharacterMovementComponent.MaxWalkSpeed` _maxvelocity (`self.CharacterMovement`))
              (set `self.damageRating` _damagerating))))
        (:`NewEnumerator1`
          (`MaterialInstanceDynamic.SetVectorParameterValue` _normalmaterial_6 "color" (struct :`R` 0.01 :`G` 0.01 :`B` 0.01 :`A` 1.0))
          (`PrimitiveComponent.SetMaterial` _mesh_4 0 _normalmaterial_6)
          (`PrimitiveComponent.SetMaterial` _mesh_4 1 "/Game/material/材质_003.材质_003")
          (bind _returnvalue_4 (`|GetDataTableRow` "/Game/util/EnemyDataTable.EnemyDataTable" "artilleryB")
            (:`then`
              (bind (_type_2 _maxhp_2 _maxmp_2 _attribute_2 _maxvelocity_2 _damagerating_2) (break `/Game/util/EnemyInfo` _returnvalue_4))
              (bind _output_get_2 (set `self.maxhp` _maxhp_2))
              (set `self.hp` _output_get_2)
              (set `self.maxmp` _maxmp_2)
              (set `CharacterMovementComponent.MaxWalkSpeed` _maxvelocity_2 (`self.CharacterMovement`))
              (set `self.damageRating` _damagerating_2))))))
    (:`NewEnumerator1`
      (`SkinnedMeshComponent.SetSkinnedAssetAndUpdate` _mesh_3 "/Game/mesh/enemy1.enemy1" true)
      (`SkeletalMeshComponent.SetAnimInstanceClass` _mesh_3 "/Game/mesh/enemy1_Skeleton_AnimBlueprint.enemy1_Skeleton_AnimBlueprint_C")
      (`SceneComponent.K2_SetRelativeLocation` _mesh_3 (0.0 0.0 -40.0) false false)
      (switch `/Game/util/Attribute` (`self.EnemyAttribute`)
        (:`NewEnumerator0`
          (`MaterialInstanceDynamic.SetVectorParameterValue` _normalmaterial_4 "color" (struct :`R` 0.99 :`G` 0.99 :`B` 0.99 :`A` 1.0))
          (`PrimitiveComponent.SetMaterial` _mesh_3 0 _normalmaterial_4)
          (`PrimitiveComponent.SetMaterial` _mesh_3 1 "/Game/material/M_PureColor_Orange.M_PureColor_Orange")
          (bind _returnvalue_5 (`|GetDataTableRow` "/Game/util/EnemyDataTable.EnemyDataTable" "infantryW")
            (:`then`
              (bind (_type_3 _maxhp_3 _maxmp_3 _attribute_3 _maxvelocity_3 _damagerating_3) (break `/Game/util/EnemyInfo` _returnvalue_5))
              (bind _output_get_3 (set `self.maxhp` _maxhp_3))
              (set `self.hp` _output_get_3)
              (set `self.maxmp` _maxmp_3)
              (set `CharacterMovementComponent.MaxWalkSpeed` _maxvelocity_3 (`self.CharacterMovement`))
              (set `self.damageRating` _damagerating_3))))
        (:`NewEnumerator1`
          (`MaterialInstanceDynamic.SetVectorParameterValue` _normalmaterial_5 "color" (struct :`R` 0.01 :`G` 0.01 :`B` 0.01 :`A` 1.0))
          (`PrimitiveComponent.SetMaterial` _mesh_3 0 _normalmaterial_5)
          (`PrimitiveComponent.SetMaterial` _mesh_3 1 "/Game/material/M_PureColor_Orange.M_PureColor_Orange")
          (bind _returnvalue_6 (`|GetDataTableRow` "/Game/util/EnemyDataTable.EnemyDataTable" "infantryB")
            (:`then`
              (bind (_type_4 _maxhp_4 _maxmp_4 _attribute_4 _maxvelocity_4 _damagerating_4) (break `/Game/util/EnemyInfo` _returnvalue_6))
              (bind _output_get_4 (set `self.maxhp` _maxhp_4))
              (set `self.hp` _output_get_4)
              (set `self.maxmp` _maxmp_4)
              (set `CharacterMovementComponent.MaxWalkSpeed` _maxvelocity_4 (`self.CharacterMovement`))
              (set `self.damageRating` _damagerating_4))))))
    (:`NewEnumerator2`
      (`SkinnedMeshComponent.SetSkinnedAssetAndUpdate` _mesh "/Game/mesh/TwinEnemy.TwinEnemy" true :!label _label)
      (`SkeletalMeshComponent.SetAnimInstanceClass` _mesh "/Game/mesh/TwinEnemy_Skeleton_AnimBlueprint.TwinEnemy_Skeleton_AnimBlueprint_C")
      (`SceneComponent.K2_SetRelativeLocation` _mesh (0.0 0.0 0.0) false false)
      (`SceneComponent.K2_SetRelativeRotation` _mesh (struct :`Yaw` 180.0) false false)
      (switch `/Game/util/Attribute` (`self.EnemyAttribute`)
        (:`NewEnumerator0`
          (`MaterialInstanceDynamic.SetVectorParameterValue` _normalmaterial_7 "color" (struct :`R` 0.99 :`G` 0.99 :`B` 0.99 :`A` 1.0))
          (`PrimitiveComponent.SetMaterial` _mesh 0 _normalmaterial_7)
          (`PrimitiveComponent.SetMaterial` _mesh 1 "/Game/material/材质.材质")
          (`PrimitiveComponent.SetMaterial` _mesh 2 "/Engine/EditorMaterials/WidgetMaterial_Z.WidgetMaterial_Z")
          (`PrimitiveComponent.SetMaterial` _mesh 3 "/Engine/EditorMaterials/WidgetMaterial_Z.WidgetMaterial_Z")
          (bind _returnvalue_7 (`|GetDataTableRow` "/Game/util/EnemyDataTable.EnemyDataTable" "GeminiW")
            (:`then`
              (bind (_type_5 _maxhp_5 _maxmp_5 _attribute_5 _maxvelocity_5 _damagerating_5) (break `/Game/util/EnemyInfo` _returnvalue_7))
              (bind _output_get_5 (set `self.maxhp` _maxhp_5))
              (set `self.hp` _output_get_5)
              (set `self.maxmp` _maxmp_5)
              (set `CharacterMovementComponent.MaxWalkSpeed` _maxvelocity_5 (`self.CharacterMovement`))
              (set `self.damageRating` _damagerating_5))))
        (:`NewEnumerator1`
          (`MaterialInstanceDynamic.SetVectorParameterValue` _normalmaterial_8 "color" (struct :`R` 0.01 :`G` 0.01 :`B` 0.01 :`A` 1.0))
          (`PrimitiveComponent.SetMaterial` _mesh 0 _normalmaterial_8)
          (`PrimitiveComponent.SetMaterial` _mesh 1 "/Game/material/材质.材质")
          (`PrimitiveComponent.SetMaterial` _mesh 2 "/Engine/EditorMaterials/WidgetMaterial_Z.WidgetMaterial_Z")
          (`PrimitiveComponent.SetMaterial` _mesh 3 "/Engine/EditorMaterials/WidgetMaterial_Z.WidgetMaterial_Z")
          (bind _returnvalue_8 (`|GetDataTableRow` "/Game/util/EnemyDataTable.EnemyDataTable" "GeminiB")
            (:`then`
              (bind (_type_6 _maxhp_6 _maxmp_6 _attribute_6 _maxvelocity_6 _damagerating_6) (break `/Game/util/EnemyInfo` _returnvalue_8))
              (bind _output_get_6 (set `self.maxhp` _maxhp_6))
              (set `self.hp` _output_get_6)
              (set `self.maxmp` _maxmp_6)
              (set `CharacterMovementComponent.MaxWalkSpeed` _maxvelocity_6 (`self.CharacterMovement`))
              (set `self.damageRating` _damagerating_6))))))
    (:`NewEnumerator3`
      (goto _label))
    (:`NewEnumerator4`
      (`SkinnedMeshComponent.SetSkinnedAssetAndUpdate` _mesh_2 "/Game/mesh/enemy3.enemy3" true)
      (`SkeletalMeshComponent.SetAnimInstanceClass` _mesh_2 "/Game/mesh/enemy3_Skeleton_AnimBlueprint.enemy3_Skeleton_AnimBlueprint_C")
      (`SceneComponent.K2_SetRelativeTransform` _mesh_2 (`KismetMathLibrary.MakeTransform` (0.0 0.0 -20.0) (struct :`Yaw` 90.0) (0.5 0.5 0.5)) false false)
      (switch `/Game/util/Attribute` (`self.EnemyAttribute`)
        (:`NewEnumerator0`
          (`MaterialInstanceDynamic.SetVectorParameterValue` _normalmaterial_2 "color" (struct :`R` 0.99 :`G` 0.99 :`B` 0.99 :`A` 1.0))
          (`PrimitiveComponent.SetMaterial` _mesh_2 0 _normalmaterial_2)
          (bind _returnvalue_9 (`|GetDataTableRow` "/Game/util/EnemyDataTable.EnemyDataTable" "ChargerW")
            (:`then`
              (bind (_type_7 _maxhp_7 _maxmp_7 _attribute_7 _maxvelocity_7 _damagerating_7) (break `/Game/util/EnemyInfo` _returnvalue_9))
              (bind _output_get_7 (set `self.maxhp` _maxhp_7))
              (set `self.hp` _output_get_7)
              (set `self.maxmp` _maxmp_7)
              (set `CharacterMovementComponent.MaxWalkSpeed` _maxvelocity_7 (`self.CharacterMovement`))
              (set `self.damageRating` _damagerating_7))))
        (:`NewEnumerator1`
          (`MaterialInstanceDynamic.SetVectorParameterValue` _normalmaterial_3 "color" (struct :`R` 0.01 :`G` 0.01 :`B` 0.01 :`A` 1.0))
          (`PrimitiveComponent.SetMaterial` _mesh_2 0 _normalmaterial_3)
          (bind _returnvalue_10 (`|GetDataTableRow` "/Game/util/EnemyDataTable.EnemyDataTable" "ChargerB")
            (:`then`
              (bind (_type_8 _maxhp_8 _maxmp_8 _attribute_8 _maxvelocity_8 _damagerating_8) (break `/Game/util/EnemyInfo` _returnvalue_10))
              (bind _output_get_8 (set `self.maxhp` _maxhp_8))
              (set `self.hp` _output_get_8)
              (set `self.maxmp` _maxmp_8)
              (set `CharacterMovementComponent.MaxWalkSpeed` _maxvelocity_8 (`self.CharacterMovement`))
              (set `self.damageRating` _damagerating_8))))))))