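; BP_PropHPReturn is a healing prop that restores the player character's HP when its influence is applied.
; It overrides the parent's AddInflunce, reads the "Heal" row from PropsDataTable and adds its Influence to HP, clamped between zero and MaxHP.
; It then shows a UMG_Description widget with the row's name and description, stores it as the character's PropUI and sets a timer for the character's UIShowEnd.
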(fn `addInflunce`
  (`parent.addInflunce`)
  (bind _asbp_character (cast `/Game/character/BP_Character` (`GameplayStatics.GetPlayerCharacter` 0)))
  (bind _returnvalue (`|GetDataTableRow` "/Game/util/PropsDataTable.PropsDataTable" "Heal")
    (:`then`
      (bind (_type _name _describe _influence) (break `/Game/util/PropsInfo` _returnvalue))
      (set `/Game/character/BP_Character.hp` (`KismetMathLibrary.FClamp` (+ (`/Game/character/BP_Character.hp` _asbp_character) _influence) 0.0 (`/Game/character/BP_Character.maxHP` _asbp_character)) _asbp_character)
      (bind _returnvalue_2 (`|CreateWidget` "/Game/UI/UMG_Description.UMG_Description_C" (`GameplayStatics.GetPlayerController` 0)))
      (set `/Game/UI/UMG_Description.Name` _name _returnvalue_2)
      (set `/Game/UI/UMG_Description.Description` _describe _returnvalue_2)
      (`UserWidget.AddToViewport` _returnvalue_2 0)
      (bind _asbp_character_2 (cast `/Game/character/BP_Character` (`GameplayStatics.GetPlayerCharacter` 0)))
      (set `/Game/character/BP_Character.PropUI` _returnvalue_2 _asbp_character_2)
      (`KismetSystemLibrary.K2_SetTimer` _asbp_character_2 "UIShowEnd" 2.0))))

(fn `UserConstructionScript`
  (`parent.UserConstructionScript`))