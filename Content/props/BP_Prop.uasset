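; BP_Prop is a pickup prop that shows a press-F prompt when the player character comes near.
; Box overlap with BP_Character sets IsCharacterChoosed and adds the UMG_PressF widget, and leaving clears the flag and removes the widget.
; The pickUp event, not triggered within this Blueprint, calls AddInflunce, plays a collect sound and destroys the actor.
; AddInflunce is empty here, so the prop itself applies no effect.
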(event `self.Box.OnComponentBeginOverlap`
  (params (OverlappedComponent :type "PrimitiveComponent Object Reference") (OtherActor :type "Actor Object Reference") (OtherComp :type "PrimitiveComponent Object Reference") (OtherBodyIndex :type Integer) (bFromSweep :type Boolean) (SweepResult :type "HitResult Structure (by ref)"))
  (cast `/Game/character/BP_Character` OtherActor)
  (set `self.isCharacterChoosed` true)
  (bind _returnvalue (`|CreateWidget` "/Game/UI/UMG_PressF.UMG_PressF_C" (`GameplayStatics.GetPlayerController` 0)))
  (`UserWidget.AddToViewport` _returnvalue 0))

(event `self.Box.OnComponentEndOverlap`
  (params (OverlappedComponent :type "PrimitiveComponent Object Reference") (OtherActor :type "Actor Object Reference") (OtherComp :type "PrimitiveComponent Object Reference") (OtherBodyIndex :type Integer))
  (cast `/Game/character/BP_Character` OtherActor)
  (set `self.isCharacterChoosed` false)
  (`Widget.RemoveFromParent` (stale `self.Box.OnComponentBeginOverlap` _returnvalue)))

(event `pickUp`
  (`self.addInflunce`)
  (`GameplayStatics.PlaySoundAtLocation` "/Game/Retro_8Bit_Sounds/Powerup/Cues/powerup_collect.powerup_collect" (`self.K2_GetActorLocation`) (struct) 1.0 1.0 0.0 null null null)
  (`self.K2_DestroyActor`))

(fn `addInflunce`)

(fn `UserConstructionScript`)